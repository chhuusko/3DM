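; Enemy AI that wanders to random nearby points, chases the player character on sight and damages it on overlap with its attack area.
; Tick issues delayed wander moves while CanSeePlayer is false; PawnSensing starts the chase, which clears that flag after a retriggerable delay.
; Two DoOnce gates re-arm each other so chase start and end sounds alternate.
; A looping timer draws the sight cone for debugging.
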(event `self.ReceiveBeginPlay`
  (`KismetSystemLibrary.K2_SetTimerDelegate` (delegate `DrawSightRadius`) 0.01 true true))

(event `DrawSightRadius`
  (`KismetSystemLibrary.DrawDebugConeInDegrees` (- (`self.K2_GetActorLocation`) (0.0 0.0 85.0)) (`self.GetActorForwardVector`) (`PawnSensingComponent.SightRadius` (`self.PawnSensing`)) (`PawnSensingComponent.PeripheralVisionAngle` (`self.PawnSensing`)) 0.0 100 (struct :`R` 1.0 :`G` 0.026042 :`B` 0.026042 :`A` 1.0) 0.0 1.0))

(event `self.ReceiveTick`
  (params (DeltaSeconds :type "Float (single-precision)"))
  (if (not (`self.CanSeePlayer?`))
    (`KismetSystemLibrary.Delay` (`KismetMathLibrary.RandomFloatInRange` 3.0 5.0))
    (if (not (`self.CanSeePlayer?`))
      (`|AIMoveTo` self (`NavigationSystemV1.K2_GetRandomReachablePointInRadius` (`self.K2_GetActorLocation`) 500.0 null null) null
        (:`then`
          (`/Engine/EditorBlueprintResources/StandardMacros.DoOnce` false :!label _label
            (:`Completed`
              (`GameplayStatics.PlaySound2D` "/Game/Audio/ChaseEnding.ChaseEnding" 1.0 1.0 0.0 null null)
              (goto _label_2 :!via `Reset`))))))))

(event `self.PawnSensing.OnSeePawn`
  (params (Pawn :type "Pawn Object Reference"))
  (`/Engine/EditorBlueprintResources/StandardMacros.DoOnce` false :!label _label_2
    (:`Completed`
      (`GameplayStatics.PlaySound2D` "/Game/Audio/ChaseStarting.ChaseStarting" 1.0 1.0 0.0 null null)
      (bind _asbp_third_person_character (cast `/Game/ThirdPerson/Blueprints/BP_ThirdPersonCharacter` Pawn))
      (`|ExecutionSequence`
        (:`then_0`
          (set `self.CanSeePlayer?` true)
          (`|AIMoveTo` self (0.0 0.0 0.0) _asbp_third_person_character
            (:`then`
              (goto _label :!via `Reset`))))
        (:`then_1`
          (`KismetSystemLibrary.RetriggerableDelay` 0.5)
          (set `self.CanSeePlayer?` false))))))

(event `self.AttackArea.OnComponentBeginOverlap`
  (params (OverlappedComponent :type "PrimitiveComponent Object Reference") (OtherActor :type "Actor Object Reference") (OtherComp :type "PrimitiveComponent Object Reference") (OtherBodyIndex :type Integer) (bFromSweep :type Boolean) (SweepResult :type "HitResult Structure (by ref)"))
  (cast `/Game/ThirdPerson/Blueprints/BP_ThirdPersonCharacter` OtherActor)
  (`GameplayStatics.ApplyDamage` (`GameplayStatics.GetPlayerCharacter` 0) 1.0)
  (`GameplayStatics.PlaySound2D` "/Game/Audio/DeathGrunt.DeathGrunt" 1.0 1.0 0.0 null null))

(fn `UserConstructionScript`)