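; BP_Ring is an interactable actor whose Ring component turns when the player uses it, with a prompt widget shown inside InteractionArea.
; Interact line-traces a short distance from the player's follow camera and requires a component tagged "Ring".
; MoveComponentTo eases the yaw, targeting the ring's world Z location plus an offset rather than its current rotation.
; A DoOnce blocks repeat input until shortly after the move completes.
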(event `self.ReceiveBeginPlay`
  (bind _asbp_third_person_character (cast `/Game/ThirdPerson/Blueprints/BP_ThirdPersonCharacter` (`GameplayStatics.GetPlayerCharacter` 0)))
  (set `self.Char Ref` _asbp_third_person_character))

(event `/Game/Blueprints/InteractInterface.Interact`
  (params (Player :type "Character Object Reference"))
  (bind _ring (`self.Ring`))
  (bind (_returnvalue_x _returnvalue_y _returnvalue_z) (`KismetMathLibrary.BreakVector` (`SceneComponent.K2_GetComponentLocation` _ring)))
  (bind _followcamera (`/Game/ThirdPerson/Blueprints/BP_ThirdPersonCharacter.FollowCamera` (`self.Char Ref`)))
  (bind _returnvalue (`SceneComponent.K2_GetComponentLocation` _followcamera))
  (bind (_returnvalue_roll _returnvalue_pitch _returnvalue_yaw) (`KismetMathLibrary.BreakRotator` (`KismetMathLibrary.MakeRotator` 0.0 0.0 (+ _returnvalue_z 90.0))))
  (bind (_outhit _returnvalue_2) (`KismetSystemLibrary.LineTraceSingle` :`Start` _returnvalue :`End` (+ _returnvalue (* (`SceneComponent.GetForwardVector` _followcamera) 200.0)) :`TraceChannel` "TraceTypeQuery1" :`bIgnoreSelf` false))
  (if _returnvalue_2
    (if (`ActorComponent.ComponentHasTag` (`.HitComponent` (`GameplayStatics.BreakHitResult` _outhit)) "Ring")
      (`/Engine/EditorBlueprintResources/StandardMacros.DoOnce` false :!label _label
        (:`Completed`
          (`KismetSystemLibrary.MoveComponentTo` (`self.Ring`) (`SceneComponent.RelativeLocation` _ring) (`KismetMathLibrary.MakeRotator` 0.0 0.0 _returnvalue_yaw) true true 1.0)
          (`KismetSystemLibrary.Delay` 0.2)
          (goto _label :!via `Reset`))))))

(event `self.InteractionArea.OnComponentBeginOverlap`
  (params (OverlappedComponent :type "PrimitiveComponent Object Reference") (OtherActor :type "Actor Object Reference") (OtherComp :type "PrimitiveComponent Object Reference") (OtherBodyIndex :type Integer) (bFromSweep :type Boolean) (SweepResult :type "HitResult Structure (by ref)"))
  (cast `/Game/ThirdPerson/Blueprints/BP_ThirdPersonCharacter` OtherActor)
  (bind _returnvalue (`|CreateWidget` "/Game/Blueprints/WBP_InteractionPrompt.WBP_InteractionPrompt_C"))
  (set `self.InteractionWidget` _returnvalue)
  (`UserWidget.AddToViewport` _returnvalue 0))

(event `self.InteractionArea.OnComponentEndOverlap`
  (params (OverlappedComponent :type "PrimitiveComponent Object Reference") (OtherActor :type "Actor Object Reference") (OtherComp :type "PrimitiveComponent Object Reference") (OtherBodyIndex :type Integer))
  (cast `/Game/ThirdPerson/Blueprints/BP_ThirdPersonCharacter` OtherActor)
  (`Widget.RemoveFromParent` (`self.InteractionWidget`)))

(fn `UserConstructionScript`)