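; Puzzle stone actor that moves along its vertical axis when its MoveStone event fires, carrying a button and a target with it.
; On BeginPlay it attaches both child components to the stone mesh, keeping world transforms, and caches the stone's starting location.
; MoveStone plays a sound at that location and runs a timeline that drives the mesh's relative Z, then calls SetLocation on the button when finished.
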(event `self.ReceiveBeginPlay`
  (bind _stonemesh (`self.StoneMesh`))
  (`self.K2_AttachToComponent` (`self.ButtonChild`) _stonemesh "None" "KeepWorld" "KeepWorld" "KeepWorld" true)
  (`self.K2_AttachToComponent` (`self.TargetChild`) _stonemesh "None" "KeepWorld" "KeepWorld" "KeepWorld" true)
  (set `self.InitialStoneLocation` (`SceneComponent.K2_GetComponentLocation` (`self.StoneMesh`))))

(event `MoveStone`
  (`GameplayStatics.PlaySoundAtLocation` "/Game/Audio/StoneMoving1Sec.StoneMoving1Sec" (`self.InitialStoneLocation`) (struct) 1.0 1.0 0.0 null null null null)
  (bind (_direction _stoneposition) (`Timeline|StoneMoving`)
    (:`Update`
      (`SceneComponent.K2_SetRelativeLocation` (`self.StoneMesh`) (`KismetMathLibrary.MakeVector` 0.0 0.0 _stoneposition) false false))
    (:`Finished`
      (`/Game/Blueprints/BP_Button.SetLocation` (`self.ButtonChild`)))))

(fn `UserConstructionScript`)