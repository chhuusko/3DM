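; Elevator actor that travels between its starting location and that location plus a MoveOffset, raised and lowered through LiftElevator and LowerElevator events.
; At BeginPlay it stores the root's world location and attaches SwitchChild to the root, keeping world transform, so it rides along.
; A single Timeline plays or reverses to lerp the root's position, with a forward or reversed sound played at the starting location.
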(event `self.ReceiveBeginPlay`
  (set `self.Initial Elevator Location` (`SceneComponent.K2_GetComponentLocation` (`self.DefaultSceneRoot`)))
  (`self.K2_AttachToComponent` (`self.SwitchChild`) (`self.DefaultSceneRoot`) "None" "KeepWorld" "KeepWorld" "KeepWorld" true))

(event `Lift Elevator`
  (`GameplayStatics.PlaySoundAtLocation` "/Game/Audio/Elevator2sec.Elevator2sec" (`self.Initial Elevator Location`) (struct) 1.0 1.0 0.0 null null null null)
  (bind (_direction _opentrack) (`Timeline|Timeline` :!label _label)
    (:`Update`
      (`SceneComponent.K2_SetWorldLocation` (`self.DefaultSceneRoot`) (`KismetMathLibrary.VLerp` (`self.Initial Elevator Location`) (+ (`self.Initial Elevator Location`) (`self.Move Offset`)) _opentrack) false false))))

(event `Lower Elevator`
  (`GameplayStatics.PlaySoundAtLocation` "/Game/Audio/Elevator2secReversed.Elevator2secReversed" (`self.Initial Elevator Location`) (struct) 1.0 1.0 0.0 null null null null)
  (goto _label :!via `Reverse`))

(fn `UserConstructionScript`)