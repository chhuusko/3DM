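; BP_MoonSecret is a one-shot hidden secret button that the third-person character can interact with.
; Its interaction area shows a prompt widget on overlap until the secret is found, and removes it when the character leaves.
; Interact sets the found flag and runs a timeline that slides the mesh by a fixed world-space offset.
; When the timeline finishes, a secret message widget appears with a sound and is removed after a short delay.
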(event `self.ReceiveBeginPlay`
  (set `self.InitalButtonLocation` (`SceneComponent.K2_GetComponentLocation` (`self.StaticMesh`)))
  (set `self.MoveOffset` (-10.0 0.0 10.0)))

(event `self.Interact`
  (params (Player :type "Character Object Reference"))
  (if (not (`self.SecretHasBeenFound`))
    (set `self.SecretHasBeenFound` true)
    (cast `/Game/ThirdPerson/Blueprints/BP_ThirdPersonCharacter` Player)
    (bind (_direction _opentrack) (`Timeline|Timeline`)
      (:`Update`
        (`SceneComponent.K2_SetWorldLocation` (`self.StaticMesh`) (`KismetMathLibrary.VLerp` (`self.InitalButtonLocation`) (+ (`self.InitalButtonLocation`) (`self.MoveOffset`)) _opentrack) false false))
      (:`Finished`
        (bind _returnvalue (`|CreateWidget` "/Game/Blueprints/WBP_SecretMessage.WBP_SecretMessage_C"))
        (set `self.SecretWidget` _returnvalue)
        (`UserWidget.AddToViewport` _returnvalue 0)
        (`GameplayStatics.PlaySound2D` "/Game/Audio/SecretFound.SecretFound" 1.0 1.0 0.0 null null)
        (`KismetSystemLibrary.Delay` 3.0)
        (`Widget.RemoveFromParent` (`self.SecretWidget`))))))

(event `self.InteractionArea.OnComponentBeginOverlap`
  (params (OverlappedComponent :type "PrimitiveComponent Object Reference") (OtherActor :type "Actor Object Reference") (OtherComp :type "PrimitiveComponent Object Reference") (OtherBodyIndex :type Integer) (bFromSweep :type Boolean) (SweepResult :type "HitResult Structure (by ref)"))
  (if (not (`self.SecretHasBeenFound`))
    (cast `/Game/ThirdPerson/Blueprints/BP_ThirdPersonCharacter` OtherActor)
    (bind _returnvalue (`|CreateWidget` "/Game/Blueprints/WBP_InteractionPrompt.WBP_InteractionPrompt_C"))
    (set `self.InteractionWidget` _returnvalue)
    (`UserWidget.AddToViewport` _returnvalue 0)))

(event `self.InteractionArea.OnComponentEndOverlap`
  (params (OverlappedComponent :type "PrimitiveComponent Object Reference") (OtherActor :type "Actor Object Reference") (OtherComp :type "PrimitiveComponent Object Reference") (OtherBodyIndex :type Integer))
  (cast `/Game/ThirdPerson/Blueprints/BP_ThirdPersonCharacter` OtherActor)
  (`Widget.RemoveFromParent` (`self.InteractionWidget`)))

(fn `UserConstructionScript`)