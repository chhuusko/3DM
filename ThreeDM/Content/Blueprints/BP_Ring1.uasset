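; BP_Ring1 is an interactable ring that yaws its static mesh by a set interval when Interact is called.
; Interact computes the target yaw and plays a Timeline that drives a Lerp on relative rotation.
; CurrentRotation is set to the target on every Update, so the Lerp collapses after the first tick.
; InteractionArea overlaps with BP_ThirdPersonCharacter add and remove the WBP_InteractionPrompt widget.
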(event `self.Interact`
  (params (Player :type "Character Object Reference"))
  (set `self.TargetRotation` (+ (`self.RotationIntervall`) (`self.CurrentRotation`)))
  (bind (_direction _newtrack_0) (`Timeline|Timeline`)
    (:`Update`
      (`SceneComponent.K2_SetRelativeRotation` (`self.StaticMesh`) (`KismetMathLibrary.MakeRotator` 0.0 0.0 (`KismetMathLibrary.Lerp` (`KismetMathLibrary.Conv_IntToDouble` (`self.CurrentRotation`)) (`KismetMathLibrary.Conv_IntToDouble` (`self.TargetRotation`)) _newtrack_0)) false false)
      (set `self.CurrentRotation` (`self.TargetRotation`)))))

(event `self.InteractionArea.OnComponentBeginOverlap`
  (params (OverlappedComponent :type "PrimitiveComponent Object Reference") (OtherActor :type "Actor Object Reference") (OtherComp :type "PrimitiveComponent Object Reference") (OtherBodyIndex :type Integer) (bFromSweep :type Boolean) (SweepResult :type "HitResult Structure (by ref)"))
  (cast `/Game/ThirdPerson/Blueprints/BP_ThirdPersonCharacter` OtherActor)
  (bind _returnvalue (`|CreateWidget` "/Game/Blueprints/WBP_InteractionPrompt.WBP_InteractionPrompt_C"))
  (set `self.InteractionWidget` _returnvalue)
  (`UserWidget.AddToViewport` _returnvalue 0))

(event `self.InteractionArea.OnComponentEndOverlap`
  (params (OverlappedComponent :type "PrimitiveComponent Object Reference") (OtherActor :type "Actor Object Reference") (OtherComp :type "PrimitiveComponent Object Reference") (OtherBodyIndex :type Integer))
  (cast `/Game/ThirdPerson/Blueprints/BP_ThirdPersonCharacter` OtherActor)
  (`Widget.RemoveFromParent` (`self.InteractionWidget`)))

(fn `UserConstructionScript`)