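; Pressure plate for an ordered-sequence puzzle that fires once on overlap and raises or lowers a linked stone.
; A plate matching CurrentStepInOrder increments that counter, lifts its stone and moves its switch through a timeline; a mismatch lowers the stone and calls ResetSequence.
; ResetSequence loops over all plates gathered on BeginPlay, but as wired only clears this plate's own activation and counter and reverses its timeline.
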(event `self.ReceiveActorBeginOverlap`
  (params (OtherActor :type "Actor Object Reference"))
  (if (not (`self.IsActivated`))
    (set `self.IsActivated` true)
    (if (== (`self.PlateInOrder`) (`self.CurrentStepInOrder`))
      (`/Engine/EditorBlueprintResources/StandardMacros.IncrementInt` (`self.CurrentStepInOrder`)
        (:`  `
          (`/Game/Blueprints/BP_StoneInOrder.MoveStoneUp` (`self.StoneToActivate`))
          (`KismetSystemLibrary.PrintString` (`KismetStringLibrary.Conv_IntToString` (`self.CurrentStepInOrder`)))
          (bind (_direction _switchposition) (`Timeline|SwitchActivate` :!label _label)
            (:`Update`
              (`SceneComponent.K2_SetRelativeLocation` (`self.Switch`) (`KismetMathLibrary.MakeVector` 0.0 0.0 _switchposition) false false)))))
      (else
        (`/Game/Blueprints/BP_StoneInOrder.MoveStoneDown` (`self.StoneToActivate`))
        (`self.ResetSequence`)
        (`KismetSystemLibrary.PrintString` "Reset")))))

(event `ResetSequence`
  (for _ (`self.AllPlatesInSequence`)
    (set `self.IsActivated` false)
    (set `self.CurrentStepInOrder` 0)
    (goto _label :!via `Reverse`)))

(event `self.ReceiveBeginPlay`
  (bind _outactors (`GameplayStatics.GetAllActorsOfClass` "BP_PressurePlateInOrder_C"))
  (set `self.AllPlatesInSequence` _outactors))

(fn `UserConstructionScript`)