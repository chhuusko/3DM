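; BP_ButtonEnd is an end-of-game button that shows a win message and quits the game when the third-person character interacts with it.
; Overlapping its interaction area shows a prompt widget, removed on exit through the same widget variable the win message reuses.
; Interacting adds the win message and plays a timeline that slides the mesh along world Y, reversing after a delay.
; When the timeline finishes, another short delay precedes quitting.
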(event `self.ReceiveBeginPlay`
  (set `self.InitalButtonLocation` (`SceneComponent.K2_GetComponentLocation` (`self.StaticMesh`)))
  (set `self.MoveOffset` (0.0 25.0 0.0)))

(event `self.Interact`
  (params (Player :type "Character Object Reference"))
  (cast `/Game/ThirdPerson/Blueprints/BP_ThirdPersonCharacter` Player)
  (bind _returnvalue (`|CreateWidget` "/Game/Blueprints/WBP_WinMessage.WBP_WinMessage_C"))
  (set `self.InteractionWidget` _returnvalue)
  (`UserWidget.AddToViewport` _returnvalue 0)
  (bind (_direction _opentrack) (`Timeline|Timeline` :!label _label)
    (:`Update`
      (`SceneComponent.K2_SetWorldLocation` (`self.StaticMesh`) (`KismetMathLibrary.VLerp` (`self.InitalButtonLocation`) (+ (`self.InitalButtonLocation`) (`self.MoveOffset`)) _opentrack) false false)
      (`KismetSystemLibrary.Delay` 1.2)
      (goto _label :!via `Reverse`))
    (:`Finished`
      (`KismetSystemLibrary.Delay` 2.0)
      (`KismetSystemLibrary.QuitGame` null "Quit"))))

(event `self.InteractionArea.OnComponentBeginOverlap`
  (params (OverlappedComponent :type "PrimitiveComponent Object Reference") (OtherActor :type "Actor Object Reference") (OtherComp :type "PrimitiveComponent Object Reference") (OtherBodyIndex :type Integer) (bFromSweep :type Boolean) (SweepResult :type "HitResult Structure (by ref)"))
  (cast `/Game/ThirdPerson/Blueprints/BP_ThirdPersonCharacter` OtherActor)
  (bind _returnvalue (`|CreateWidget` "/Game/Blueprints/WBP_InteractionPrompt.WBP_InteractionPrompt_C"))
  (set `self.InteractionWidget` _returnvalue)
  (`UserWidget.AddToViewport` _returnvalue 0))

(event `self.InteractionArea.OnComponentEndOverlap`
  (params (OverlappedComponent :type "PrimitiveComponent Object Reference") (OtherActor :type "Actor Object Reference") (OtherComp :type "PrimitiveComponent Object Reference") (OtherBodyIndex :type Integer))
  (cast `/Game/ThirdPerson/Blueprints/BP_ThirdPersonCharacter` OtherActor)
  (`Widget.RemoveFromParent` (`self.InteractionWidget`)))

(fn `UserConstructionScript`)