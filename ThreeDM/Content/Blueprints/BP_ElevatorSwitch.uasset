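; BP_ElevatorSwitch is an interactable switch that raises or lowers the BP_Elevator whose ElevatorValue matches its SwitchValue.
; Interact searches all elevators, toggles the matching one and plays or reverses a Timeline that tilts the switch mesh's pitch.
; After a lift finishes, a 10-second delay automatically lowers the elevator if it is not moving.
; Overlapping InteractionArea with the third-person character shows an interaction prompt widget, removed on exit.
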(event `self.ReceiveBeginPlay`
  (set `self.InitalSwitchRotation` (`KismetMathLibrary.Conv_RotatorToVector` (`SceneComponent.K2_GetComponentRotation` (`self.StaticMesh`)))))

(event `self.Interact`
  (params (Player :type "Character Object Reference"))
  (bind (_initalswitchrotation_x _initalswitchrotation_y) (`KismetMathLibrary.BreakVector` (`self.InitalSwitchRotation`)))
  (bind (_rotationoffset_x _rotationoffset_y) (`KismetMathLibrary.BreakVector` (`self.RotationOffset`)))
  (bind (_initalswitchrotation_x_2 _initalswitchrotation_y_2) (`KismetMathLibrary.BreakVector` (`self.InitalSwitchRotation`)))
  (bind _outactors (`GameplayStatics.GetAllActorsOfClass` "/Game/Blueprints/BP_Elevator.BP_Elevator_C"))
  (for _array_element _outactors
    (if (== (`/Game/Blueprints/BP_Elevator.ElevatorValue` _array_element) (`self.SwitchValue`))
      (set `self.Elevator is moving` true)
      (if (`self.Elevator is up`)
        (set `self.Elevator is up` false :!label _label)
        (`/Game/Blueprints/BP_Elevator.Lower Elevator` _array_element)
        (bind (_direction _opentrack) (`Timeline|Timeline` :!via `Reverse` :!label _label_2)
          (:`Update`
            (bind (_returnvalue_x _returnvalue_y) (`KismetMathLibrary.BreakVector` (`KismetMathLibrary.VLerp` (`KismetMathLibrary.MakeVector` 0.0 _initalswitchrotation_y_2) (+ _initalswitchrotation_y _rotationoffset_y) _opentrack)))
            (`SceneComponent.K2_SetWorldRotation` (`self.StaticMesh`) (`KismetMathLibrary.MakeRotator` 0.0 _returnvalue_y 180.0) false false))
          (:`Finished`
            (set `self.Elevator is moving` false)
            (if (`self.Elevator is up`)
              (`KismetSystemLibrary.Delay` 10.0)
              (if (not (`self.Elevator is moving`))
                (set `self.Elevator is moving` true)
                (goto _label))
              (else
                (break)))))
        (else
          (set `self.Elevator is up` true)
          (`/Game/Blueprints/BP_Elevator.Lift Elevator` _array_element)
          (goto _label_2))))))

(event `self.InteractionArea.OnComponentBeginOverlap`
  (params (OverlappedComponent :type "PrimitiveComponent Object Reference") (OtherActor :type "Actor Object Reference") (OtherComp :type "PrimitiveComponent Object Reference") (OtherBodyIndex :type Integer) (bFromSweep :type Boolean) (SweepResult :type "HitResult Structure (by ref)"))
  (cast `/Game/ThirdPerson/Blueprints/BP_ThirdPersonCharacter` OtherActor)
  (bind _returnvalue (`|CreateWidget` "/Game/Blueprints/WBP_InteractionPrompt.WBP_InteractionPrompt_C"))
  (set `self.InteractionWidget` _returnvalue)
  (`UserWidget.AddToViewport` _returnvalue 0))

(event `self.InteractionArea.OnComponentEndOverlap`
  (params (OverlappedComponent :type "PrimitiveComponent Object Reference") (OtherActor :type "Actor Object Reference") (OtherComp :type "PrimitiveComponent Object Reference") (OtherBodyIndex :type Integer))
  (cast `/Game/ThirdPerson/Blueprints/BP_ThirdPersonCharacter` OtherActor)
  (`Widget.RemoveFromParent` (`self.InteractionWidget`)))

(fn `UserConstructionScript`)