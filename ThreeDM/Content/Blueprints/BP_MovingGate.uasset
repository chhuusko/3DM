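; Moving gate Blueprint that slides a stone mesh along its relative Z axis when MoveStone is triggered.
; On BeginPlay it attaches ButtonChild and TargetChild to the stone with world transforms kept, so both ride along with it.
; The StoneMoving timeline drives the stone's position, then calls SetLocation on ButtonChild when it finishes.
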(event `self.ReceiveBeginPlay`
  (bind _stonemesh (`self.StoneMesh`))
  (`self.K2_AttachToComponent` (`self.ButtonChild`) _stonemesh "None" "KeepWorld" "KeepWorld" "KeepWorld" true)
  (`self.K2_AttachToComponent` (`self.TargetChild`) _stonemesh "None" "KeepWorld" "KeepWorld" "KeepWorld" true))

(event `MoveStone`
  (bind (_direction _stoneposition) (`Timeline|StoneMoving`)
    (:`Update`
      (`SceneComponent.K2_SetRelativeLocation` (`self.StoneMesh`) (`KismetMathLibrary.MakeVector` 0.0 0.0 _stoneposition) false false))
    (:`Finished`
      (`/Game/Blueprints/BP_Button.SetLocation` (`self.ButtonChild`)))))

(fn `UserConstructionScript`)