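; BP_PuzzlePlate is a puzzle pressure plate that the player pawn triggers by overlapping it.
; On overlap, if not already activated, it calls the Activate dispatcher with itself and plays a Timeline that moves the Switch component's relative location.
; Any end overlap reverses the Timeline, without checking the actor or the activated state.
; The Activated flag changes only through SetActiveState, which the plate itself never calls.
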(event `self.ReceiveActorBeginOverlap`
  (params (OtherActor :type "Actor Object Reference"))
  (if (and (== OtherActor (`GameplayStatics.GetPlayerPawn` 0)) (not (`self.Activated`)))
    (`self.Activate` self)
    (bind (_direction _switchposition) (`Timeline|Timeline` :!label _label)
      (:`Update`
        (`SceneComponent.K2_SetRelativeLocation` (`self.Switch`) (`KismetMathLibrary.MakeVector` 0.0 0.0 _switchposition) false false)))))

(event `self.ReceiveActorEndOverlap`
  (params (OtherActor :type "Actor Object Reference"))
  (goto _label :!via `Reverse`))

(fn `Set Active State`
  (params (Activated :type Boolean))
  (set `self.Activated` Activated))

(fn `UserConstructionScript`)