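; BP_MirrorPuzzleButton is an interactable mirror-puzzle button that opens its linked Gate.
; On BeginPlay it caches the mesh location and picks a short press offset along world X or Y from its yaw, while SetLocation can re-cache the location.
; Interact plays a sound, opens the Gate and slides the mesh by Timeline, which auto-reverses after a DoOnce-guarded delay.
; InteractionArea overlaps show and remove the player's prompt widget.
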(event `SetLocation`
  (set `self.InitalButtonLocation` (`SceneComponent.K2_GetComponentLocation` (`self.StaticMesh`))))

(event `self.ReceiveBeginPlay`
  (bind (_initialbuttonrotation_x _initialbuttonrotation_y _initialbuttonrotation_z) (`KismetMathLibrary.BreakVector` (`self.InitialButtonRotation`)))
  (bind (_initialbuttonrotation_x_2 _initialbuttonrotation_y_2 _initialbuttonrotation_z_2) (`KismetMathLibrary.BreakVector` (`self.InitialButtonRotation`)))
  (bind (_initialbuttonrotation_x_3 _initialbuttonrotation_y_3 _initialbuttonrotation_z_3) (`KismetMathLibrary.BreakVector` (`self.InitialButtonRotation`)))
  (bind (_returnvalue_roll _returnvalue_pitch _returnvalue_yaw) (`KismetMathLibrary.BreakRotator` (`SceneComponent.K2_GetComponentRotation` (`self.StaticMesh`))))
  (set `self.InitalButtonLocation` (`SceneComponent.K2_GetComponentLocation` (`self.StaticMesh`)))
  (set `self.InitialButtonRotation` (`KismetMathLibrary.Conv_DoubleToVector` _returnvalue_yaw))
  (if (`KismetMathLibrary.NearlyEqual_FloatFloat` 0.0 _initialbuttonrotation_z_2 1.0)
    (set `self.MoveOffset` (0.0 -7.5 0.0))
    (elif (`KismetMathLibrary.NearlyEqual_FloatFloat` 90.0 _initialbuttonrotation_z_3 1.0)
      (set `self.MoveOffset` (7.5 0.0 0.0))
      (elif (`KismetMathLibrary.NearlyEqual_FloatFloat` 180.0 _initialbuttonrotation_z 1.0)
        (set `self.MoveOffset` (0.0 7.5 0.0))
        (else
          (set `self.MoveOffset` (-7.5 0.0 0.0)))))))

(event `self.Interact`
  (params (Player :type "Character Object Reference"))
  (`GameplayStatics.PlaySoundAtLocation` "/Game/Audio/Button.Button" (`self.InitalButtonLocation`) (struct) 1.0 1.0 0.0 null null null null)
  (`/Game/Blueprints/BP_MirrorPuzzleGate.OpenGate` (`self.Gate`))
  (bind (_direction _opentrack) (`Timeline|Timeline` :!label _label)
    (:`Update`
      (`SceneComponent.K2_SetWorldLocation` (`self.StaticMesh`) (`KismetMathLibrary.VLerp` (`self.InitalButtonLocation`) (+ (`self.InitalButtonLocation`) (`self.MoveOffset`)) _opentrack) false false)
      (`KismetSystemLibrary.Delay` 1.2)
      (`/Engine/EditorBlueprintResources/StandardMacros.DoOnce` false :!label _label_2
        (:`Completed`
          (goto _label :!via `Reverse`))))
    (:`Finished`
      (`/Engine/EditorBlueprintResources/StandardMacros.DoOnce` false
        (:`Completed`
          (goto _label_2 :!via `Reset`))))))

(event `self.InteractionArea.OnComponentBeginOverlap`
  (params (OverlappedComponent :type "PrimitiveComponent Object Reference") (OtherActor :type "Actor Object Reference") (OtherComp :type "PrimitiveComponent Object Reference") (OtherBodyIndex :type Integer) (bFromSweep :type Boolean) (SweepResult :type "HitResult Structure (by ref)"))
  (cast `/Game/ThirdPerson/Blueprints/BP_ThirdPersonCharacter` OtherActor)
  (bind _returnvalue (`|CreateWidget` "/Game/Blueprints/WBP_InteractionPrompt.WBP_InteractionPrompt_C"))
  (set `self.InteractionWidget` _returnvalue)
  (`UserWidget.AddToViewport` _returnvalue 0))

(event `self.InteractionArea.OnComponentEndOverlap`
  (params (OverlappedComponent :type "PrimitiveComponent Object Reference") (OtherActor :type "Actor Object Reference") (OtherComp :type "PrimitiveComponent Object Reference") (OtherBodyIndex :type Integer))
  (cast `/Game/ThirdPerson/Blueprints/BP_ThirdPersonCharacter` OtherActor)
  (`Widget.RemoveFromParent` (`self.InteractionWidget`)))

(fn `UserConstructionScript`)