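; BP_BigBox is a box actor that plays a sound while it moves.
; Every Tick, it compares the static mesh component's velocity magnitude to a fixed speed threshold.
; An IsPlaying flag makes the audio start once when the speed rises above the threshold and briefly fade out when it drops back.
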(event `self.ReceiveTick`
  (params (DeltaSeconds :type "Float (single-precision)"))
  (if (> (`KismetMathLibrary.VSize` (`SceneComponent.GetComponentVelocity` (`self.StaticMesh`))) 30.0)
    (if (not (`self.IsPlaying?`))
      (`AudioComponent.Play` (`self.Audio`) 0.2)
      (set `self.IsPlaying?` true))
    (elif (`self.IsPlaying?`)
      (`AudioComponent.FadeOut` (`self.Audio`) 0.2 0.0 "Linear")
      (set `self.IsPlaying?` false))))

(fn `UserConstructionScript`)