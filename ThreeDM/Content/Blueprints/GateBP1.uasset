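; Gate actor that slides its static mesh from its starting position to an offset position when the OpenGate event is called.
; BeginPlay caches the mesh's world location as the start point.
; OpenGate plays a timeline whose OpenTrack lerps the mesh from that location to it plus MoveOffset, without sweeping; there is no close logic.
; Debug strings print at start and on every timeline update.
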(event `self.ReceiveBeginPlay`
  (bind _output_get (set `self.Initial Gate Location` (`SceneComponent.K2_GetComponentLocation` (`self.StaticMesh`))))
  (`KismetSystemLibrary.PrintString` (`KismetStringLibrary.Conv_VectorToString` _output_get)))

(event `OpenGate`
  (bind (_direction _opentrack) (`Timeline|Timeline`)
    (:`Update`
      (`SceneComponent.K2_SetWorldLocation` (`self.StaticMesh`) (`KismetMathLibrary.VLerp` (`self.Initial Gate Location`) (+ (`self.Initial Gate Location`) (`self.Move Offset`)) _opentrack) false false)
      (`KismetSystemLibrary.PrintString` "no"))))

(fn `UserConstructionScript`)