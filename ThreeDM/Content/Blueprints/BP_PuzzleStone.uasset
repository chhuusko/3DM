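; BP_PuzzleStone is a puzzle stone that moves vertically once its pressure plates are activated in the correct order.
; On BeginPlay it attaches ButtonChild to StoneMesh and binds to each referenced plate's activation event.
; The PressurePlates array order defines the sequence: a correct plate advances the counter, while a wrong one resets all plates.
; The final correct plate plays a Timeline that drives the stone's relative Z and updates the button's location.
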(event `self.ReceiveBeginPlay`
  (`self.K2_AttachToComponent` (`self.ButtonChild`) (`self.StoneMesh`) "None" "KeepWorld" "KeepWorld" "KeepWorld" true)
  (for _array_element (`self.PressurePlates`)
    (`/Engine/EditorBlueprintResources/StandardMacros.IsValid` _array_element
      (:`Is Valid`
        (add `/Game/Blueprints/BP_PuzzlePlate.Activate` _array_element (`|CreateDelegate` :!event `ActivatedPressurePlate`)))
      (:`Is Not Valid`
        (`KismetSystemLibrary.PrintString` "Add Reference!")))))

(event `ActivatedPressurePlate`
  (params (`Activated Pressure Plate` :type "/Game/Blueprints/BP_PuzzlePlate Object Reference"))
  (bind _activated_pressureplates (`self.Activated PressurePlates`))
  (if (== `Activated Pressure Plate` (`|GetArrayItem` (`self.PressurePlates`) (`self.Activated PressurePlates`)))
    (`/Game/Blueprints/BP_PuzzlePlate.Set Active State` `Activated Pressure Plate` true)
    (`KismetSystemLibrary.PrintString` (`KismetStringLibrary.Conv_IntToString` _activated_pressureplates))
    (if (== _activated_pressureplates (`KismetArrayLibrary.Array_LastIndex` (`self.PressurePlates`)))
      (bind (_direction _stoneposition) (`Timeline|Timeline`)
        (:`Update`
          (`SceneComponent.K2_SetRelativeLocation` (`self.StoneMesh`) (`KismetMathLibrary.MakeVector` 0.0 0.0 _stoneposition) false false)
          (`/Game/Blueprints/BP_Button.SetLocation` (`self.ButtonChild`))))
      (else
        (`/Engine/EditorBlueprintResources/StandardMacros.IncrementInt` _activated_pressureplates)))
    (else
      (`self.Reset Pressure Plates`))))

(fn `Reset Pressure Plates`
  (for _array_element (`self.PressurePlates`)
    (`/Game/Blueprints/BP_PuzzlePlate.Set Active State` _array_element false))
  (set `self.Activated PressurePlates` 0))

(fn `UserConstructionScript`)