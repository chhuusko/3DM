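; BP_PuzzlePillar is an interactable puzzle pillar that turns 90 degrees in yaw per interaction, carrying an attached StarActor with it.
; A timeline interpolates the rotation, while a DoOnce blocks repeat input until shortly after the turn finishes.
; Each finished turn asks the Manager to check puzzle status.
; An overlap area shows and removes an interaction prompt widget for the third-person character.
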(event `self.ReceiveBeginPlay`
  (`self.K2_AttachToComponent` (`self.Star Actor`) (`self.DefaultSceneRoot`) "None" "KeepWorld" "KeepWorld" "KeepWorld" true))

(event `/Game/Blueprints/InteractInterface.Interact`
  (params (Player :type "Character Object Reference"))
  (bind (_currentrotation_x _currentrotation_y _currentrotation_z) (`KismetMathLibrary.BreakVector` (`self.CurrentRotation`)))
  (bind (_currentrotation_x_2 _currentrotation_y_2 _currentrotation_z_2) (`KismetMathLibrary.BreakVector` (`self.CurrentRotation`)))
  (`/Engine/EditorBlueprintResources/StandardMacros.DoOnce` false :!label _label
    (:`Completed`
      (set `self.TargetRotation` (`KismetMathLibrary.MakeVector` 0.0 0.0 (+ _currentrotation_z 90.0)))
      (bind (_direction _opentrack) (`Timeline|Timeline` :!via `PlayFromStart`)
        (:`Update`
          (bind (_returnvalue_x _returnvalue_y _returnvalue_z) (`KismetMathLibrary.BreakVector` (`KismetMathLibrary.VLerp` (`self.CurrentRotation`) (`self.TargetRotation`) _opentrack)))
          (`SceneComponent.K2_SetWorldRotation` (`self.DefaultSceneRoot`) (`KismetMathLibrary.MakeRotator` 0.0 0.0 _returnvalue_z) false false))
        (:`Finished`
          (set `self.CurrentRotation` (`KismetMathLibrary.MakeVector` 0.0 0.0 (+ 90.0 _currentrotation_z_2)))
          (`/Game/Blueprints/BP_PillarPuzzleManager.CheckPuzzleStatus` (`self.Manager`))
          (`KismetSystemLibrary.Delay` 0.2)
          (goto _label :!via `Reset`))))))

(event `self.InteractionArea.OnComponentBeginOverlap`
  (params (OverlappedComponent :type "PrimitiveComponent Object Reference") (OtherActor :type "Actor Object Reference") (OtherComp :type "PrimitiveComponent Object Reference") (OtherBodyIndex :type Integer) (bFromSweep :type Boolean) (SweepResult :type "HitResult Structure (by ref)"))
  (cast `/Game/ThirdPerson/Blueprints/BP_ThirdPersonCharacter` OtherActor)
  (bind _returnvalue (`|CreateWidget` "/Game/Blueprints/WBP_InteractionPrompt.WBP_InteractionPrompt_C"))
  (set `self.InteractionWidget` _returnvalue)
  (`UserWidget.AddToViewport` _returnvalue 0))

(event `self.InteractionArea.OnComponentEndOverlap`
  (params (OverlappedComponent :type "PrimitiveComponent Object Reference") (OtherActor :type "Actor Object Reference") (OtherComp :type "PrimitiveComponent Object Reference") (OtherBodyIndex :type Integer))
  (cast `/Game/ThirdPerson/Blueprints/BP_ThirdPersonCharacter` OtherActor)
  (`Widget.RemoveFromParent` (`self.InteractionWidget`)))

(fn `UserConstructionScript`)