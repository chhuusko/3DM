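; BP_MirrorPuzzleGate is a gate for a mirror puzzle that slides open once and then triggers a light cast.
; On BeginPlay it records the mesh's location and attaches TargetChild to the mesh, keeping its world transform.
; OpenGate passes a DoOnce, plays a moving sound and uses a timeline to lerp the mesh by MoveOffset.
; When the timeline finishes, it calls CastLight on LightSource.
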(event `self.ReceiveBeginPlay`
  (set `self.Initial Gate Location` (`SceneComponent.K2_GetComponentLocation` (`self.StaticMesh`)))
  (`self.K2_AttachToComponent` (`self.TargetChild`) (`self.StaticMesh`) "None" "KeepWorld" "KeepWorld" "KeepWorld" true))

(event `OpenGate`
  (`/Engine/EditorBlueprintResources/StandardMacros.DoOnce` false
    (:`Completed`
      (`GameplayStatics.PlaySoundAtLocation` "/Game/Audio/GateMoving.GateMoving" (`self.Initial Gate Location`) (struct) 1.0 1.0 0.0 null null null null)
      (bind (_direction _opentrack) (`Timeline|Timeline`)
        (:`Update`
          (`SceneComponent.K2_SetWorldLocation` (`self.StaticMesh`) (`KismetMathLibrary.VLerp` (`self.Initial Gate Location`) (+ (`self.Initial Gate Location`) (`self.Move Offset`)) _opentrack) false false))
        (:`Finished`
          (`/Game/Blueprints/BP_LightLineTrace.CastLight` (`self.Light Source`)))))))

(fn `UserConstructionScript`)