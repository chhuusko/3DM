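; BP_Button is a pressable button actor that shows an interaction prompt to the player while they are near it.
; Overlaps on InteractionArea, filtered to BP_ThirdPersonCharacter, set PlayerInRange and create or remove the WBP_InteractionPrompt widget.
; The prompt appears only while HasBeenPressed is false, though this graph contains no logic that handles the press or sets that flag.
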(event `self.InteractionArea.OnComponentBeginOverlap`
  (params (OverlappedComponent :type "PrimitiveComponent Object Reference") (OtherActor :type "Actor Object Reference") (OtherComp :type "PrimitiveComponent Object Reference") (OtherBodyIndex :type Integer) (bFromSweep :type Boolean) (SweepResult :type "HitResult Structure (by ref)"))
  (cast `/Game/ThirdPerson/Blueprints/BP_ThirdPersonCharacter` OtherActor)
  (set `self.PlayerInRange` true)
  (if (not (`self.HasBeenPressed`))
    (bind _returnvalue (`|CreateWidget` "/Game/Blueprints/WBP_InteractionPrompt.WBP_InteractionPrompt_C"))
    (set `self.InteractionWidget` _returnvalue)
    (`UserWidget.AddToViewport` _returnvalue 0)))

(event `self.InteractionArea.OnComponentEndOverlap`
  (params (OverlappedComponent :type "PrimitiveComponent Object Reference") (OtherActor :type "Actor Object Reference") (OtherComp :type "PrimitiveComponent Object Reference") (OtherBodyIndex :type Integer))
  (cast `/Game/ThirdPerson/Blueprints/BP_ThirdPersonCharacter` OtherActor)
  (set `self.PlayerInRange` false)
  (`Widget.RemoveFromParent` (`self.InteractionWidget`)))

(fn `UserConstructionScript`)