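; Pressure plate actor that activates a linked stone while stepped on and deactivates it when the overlap ends.
; Overlap events call SwitchActivated or SwitchDeactivated on StoneToActivate and play a sound at the plate location cached on BeginPlay.
; The SwitchActivate timeline drives the Switch component's relative Z, playing forward on begin overlap and reversing on end.
; Overlaps are neither filtered nor counted, so any actor entering or leaving toggles it.
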(event `self.ReceiveBeginPlay`
  (set `self.InitialPlateLocation` (`SceneComponent.K2_GetComponentLocation` (`self.Switch`))))

(event `self.ReceiveActorBeginOverlap`
  (params (OtherActor :type "Actor Object Reference"))
  (`/Game/Blueprints/BP_MovingStone.SwitchActivated` (`self.StoneToActivate`))
  (`GameplayStatics.PlaySoundAtLocation` "/Game/Audio/PressurePlate1Sec.PressurePlate1Sec" (`self.InitialPlateLocation`) (struct) 1.0 1.0 0.0 null null null null)
  (bind (_direction _switchposition) (`Timeline|SwitchActivate` :!label _label)
    (:`Update`
      (`SceneComponent.K2_SetRelativeLocation` (`self.Switch`) (`KismetMathLibrary.MakeVector` 0.0 0.0 _switchposition) false false))))

(event `self.ReceiveActorEndOverlap`
  (params (OtherActor :type "Actor Object Reference"))
  (`/Game/Blueprints/BP_MovingStone.SwitchDeactivated` (`self.StoneToActivate`))
  (`GameplayStatics.PlaySoundAtLocation` "/Game/Audio/PressurePlate1Sec.PressurePlate1Sec" (`self.InitialPlateLocation`) (struct) 1.0 1.0 0.0 null null null null)
  (goto _label :!via `Reverse`))

(fn `UserConstructionScript`)