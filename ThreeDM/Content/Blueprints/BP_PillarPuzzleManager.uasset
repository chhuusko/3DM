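; Puzzle manager that moves a stone once the pillars in its array are rotated to their target angles.
; CheckPuzzleStatus compares each pillar's yaw to the matching TargetRotationValues entry within a small tolerance, counting matches and zeroing the count at the first mismatch.
; When the count reaches at least five, it calls MoveStone on MovingStone; the count is not reset before each check.
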(event `CheckPuzzleStatus`
  (for (_array_element _array_index) (`self.Pillars`)
    (bind (_returnvalue_roll _returnvalue_pitch _returnvalue_yaw) (`KismetMathLibrary.BreakRotator` (`self.K2_GetActorRotation` _array_element)))
    (if (`KismetMathLibrary.NearlyEqual_FloatFloat` _returnvalue_yaw (`|GetArrayItem` (`self.TargetRotationValues`) _array_index) 1.0)
      (`/Engine/EditorBlueprintResources/StandardMacros.IncrementInt` (`self.CompletedPillars`))
      (else
        (set `self.CompletedPillars` 0)
        (break))))
  (if (>= (`self.CompletedPillars`) 5)
    (`/Game/Blueprints/BP_MovingStone.MoveStone` (`self.MovingStone`))))

(fn `UserConstructionScript`)