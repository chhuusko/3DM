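; Interactable light-puzzle mirror that turns through four preset orientations and has its light source recast the light after each turn.
; Interact plays a sound, advances RotationIndex and picks a hardcoded pitch/yaw from a nested branch tree keyed on MirrorIndex.
; A Timeline lerps to that rotation, then calls CastLight, with a DoOnce blocking input until shortly afterward.
; Overlapping InteractionArea shows or removes the player's interaction prompt.
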(event `self.ReceiveBeginPlay`
  (bind (_returnvalue_roll _returnvalue_pitch _returnvalue_yaw) (`KismetMathLibrary.BreakRotator` (`SceneComponent.K2_GetComponentRotation` (`self.DefaultSceneRoot`))))
  (set `self.InitialMirrorRotation` (`KismetMathLibrary.MakeVector` 0.0 _returnvalue_pitch _returnvalue_yaw))
  (set `self.InitialMirrorPosition` (`SceneComponent.K2_GetComponentLocation` (`self.StaticMesh`))))

(event `/Game/Blueprints/InteractInterface.Interact`
  (params (Player :type "Character Object Reference"))
  (bind (_returnvalue_roll _returnvalue_pitch _returnvalue_yaw) (`KismetMathLibrary.BreakRotator` (`SceneComponent.K2_GetComponentRotation` (`self.DefaultSceneRoot`))))
  (`/Engine/EditorBlueprintResources/StandardMacros.DoOnce` false :!label _label
    (:`Completed`
      (`GameplayStatics.PlaySoundAtLocation` "/Game/Audio/MirrorRotating1Sec.MirrorRotating1Sec" (`self.InitialMirrorPosition`) (struct) 1.0 1.0 0.0 null null null null)
      (if (!= (`self.RotationIndex`) 3)
        (`/Engine/EditorBlueprintResources/StandardMacros.IncrementInt` (`self.RotationIndex`)
          (:`  `
            _))
        (else
          (set `self.RotationIndex` 0)))
      (if (== 0 (`self.MirrorIndex`))
        (if (== 0 (`self.RotationIndex`))
          (set `self.NewMirrorRotation` (0.0 1.0 -113.91545))
          (bind (_direction _opentrack) (`Timeline|Timeline` :!via `PlayFromStart` :!label _label_2)
            (:`Update`
              (bind (_returnvalue_x _returnvalue_y _returnvalue_z) (`KismetMathLibrary.BreakVector` (`KismetMathLibrary.VLerp` (`self.InitialMirrorRotation`) (`self.NewMirrorRotation`) _opentrack)))
              (`SceneComponent.K2_SetWorldRotation` (`self.DefaultSceneRoot`) (`KismetMathLibrary.MakeRotator` 0.0 _returnvalue_y _returnvalue_z) false false))
            (:`Finished`
              (set `self.InitialMirrorRotation` (`KismetMathLibrary.MakeVector` 0.0 _returnvalue_pitch _returnvalue_yaw))
              (`/Game/Blueprints/BP_LightLineTrace.CastLight` (`self.LightSource`))
              (`KismetSystemLibrary.Delay` 0.2)
              (goto _label :!via `Reset`)))
          (elif (== 1 (`self.RotationIndex`))
            (set `self.NewMirrorRotation` (0.0 2.0 -38.613516))
            (goto _label_2 :!via `PlayFromStart`)
            (elif (== 2 (`self.RotationIndex`))
              (set `self.NewMirrorRotation` (0.0 3.5 133.424509))
              (goto _label_2 :!via `PlayFromStart`)
              (else
                (set `self.NewMirrorRotation` (0.0 -0.5 139.586618))
                (goto _label_2 :!via `PlayFromStart`)))))
        (elif (== 1 (`self.MirrorIndex`))
          (if (== 0 (`self.RotationIndex`))
            (set `self.NewMirrorRotation` (0.0 3.0 -5.0))
            (goto _label_2 :!via `PlayFromStart`)
            (elif (== 1 (`self.RotationIndex`))
              (set `self.NewMirrorRotation` (0.0 5.5 117.30119))
              (goto _label_2 :!via `PlayFromStart`)
              (elif (== 2 (`self.RotationIndex`))
                (set `self.NewMirrorRotation` (0.0 2.0 114.555748))
                (goto _label_2 :!via `PlayFromStart`)
                (else
                  (set `self.NewMirrorRotation` (0.0 4.0 -90.0))
                  (goto _label_2 :!via `PlayFromStart`)))))
          (elif (== 2 (`self.MirrorIndex`))
            (if (== 0 (`self.RotationIndex`))
              (set `self.NewMirrorRotation` (0.0 10.0 40.0))
              (goto _label_2 :!via `PlayFromStart`)
              (elif (== 1 (`self.RotationIndex`))
                (set `self.NewMirrorRotation` (0.0 7.0 -58.019482))
                (goto _label_2 :!via `PlayFromStart`)
                (elif (== 2 (`self.RotationIndex`))
                  (set `self.NewMirrorRotation` (0.0 9.0 130.0))
                  (goto _label_2 :!via `PlayFromStart`)
                  (else
                    (set `self.NewMirrorRotation` (0.0 13.3 -60.451536))
                    (goto _label_2 :!via `PlayFromStart`)))))
            (elif (== 3 (`self.MirrorIndex`))
              (if (== 0 (`self.RotationIndex`))
                (set `self.NewMirrorRotation` (0.0 -3.18 2.73))
                (goto _label_2 :!via `PlayFromStart`)
                (elif (== 1 (`self.RotationIndex`))
                  (set `self.NewMirrorRotation` (0.0 -5.1 8.04))
                  (goto _label_2 :!via `PlayFromStart`)
                  (elif (== 2 (`self.RotationIndex`))
                    (set `self.NewMirrorRotation` (0.0 -1.85 10.3))
                    (goto _label_2 :!via `PlayFromStart`)
                    (else
                      (set `self.NewMirrorRotation` (0.0 0.5 5.027317))
                      (goto _label_2 :!via `PlayFromStart`)))))
              (elif (== 4 (`self.MirrorIndex`))
                (if (== 0 (`self.RotationIndex`))
                  (set `self.NewMirrorRotation` (0.0 2.28 3.001352))
                  (goto _label_2 :!via `PlayFromStart`)
                  (elif (== 1 (`self.RotationIndex`))
                    (set `self.NewMirrorRotation` (0.0 4.1 9.72))
                    (goto _label_2 :!via `PlayFromStart`)
                    (elif (== 2 (`self.RotationIndex`))
                      (set `self.NewMirrorRotation` (0.0 0.2 7.820494))
                      (goto _label_2 :!via `PlayFromStart`)
                      (else
                        (set `self.NewMirrorRotation` (0.0 6.75 4.93))
                        (goto _label_2 :!via `PlayFromStart`)))))
                (elif (== 5 (`self.MirrorIndex`))
                  (if (== 0 (`self.RotationIndex`))
                    (set `self.NewMirrorRotation` (0.0 2.0 120.0))
                    (goto _label_2 :!via `PlayFromStart`)
                    (elif (== 1 (`self.RotationIndex`))
                      (set `self.NewMirrorRotation` (0.0 3.0 10.0))
                      (goto _label_2 :!via `PlayFromStart`)
                      (elif (== 2 (`self.RotationIndex`))
                        (set `self.NewMirrorRotation` (0.0 4.3 -101.8))
                        (goto _label_2 :!via `PlayFromStart`)
                        (else
                          (set `self.NewMirrorRotation` (0.0 1.5 -98.359073))
                          (goto _label_2 :!via `PlayFromStart`)))))
                  (elif (== 6 (`self.MirrorIndex`))
                    (if (== 0 (`self.RotationIndex`))
                      (set `self.NewMirrorRotation` (0.0 4.0 -20.0))
                      (goto _label_2 :!via `PlayFromStart`)
                      (elif (== 1 (`self.RotationIndex`))
                        (set `self.NewMirrorRotation` (0.0 8.0 69.12))
                        (goto _label_2 :!via `PlayFromStart`)
                        (elif (== 2 (`self.RotationIndex`))
                          (set `self.NewMirrorRotation` (0.0 14.0 -110.0))
                          (goto _label_2 :!via `PlayFromStart`)
                          (else
                            (set `self.NewMirrorRotation` (0.0 19.0 73.4))
                            (goto _label_2 :!via `PlayFromStart`)))))
                    (elif (== 7 (`self.MirrorIndex`))
                      (if (== 0 (`self.RotationIndex`))
                        (set `self.NewMirrorRotation` (0.0 2.0 160.0))
                        (goto _label_2 :!via `PlayFromStart`)
                        (elif (== 1 (`self.RotationIndex`))
                          (set `self.NewMirrorRotation` (0.0 3.4 -18.7))
                          (goto _label_2 :!via `PlayFromStart`)
                          (elif (== 2 (`self.RotationIndex`))
                            (set `self.NewMirrorRotation` (0.0 1.3 40.0))
                            (goto _label_2 :!via `PlayFromStart`)
                            (else
                              (set `self.NewMirrorRotation` (0.0 -0.5 -3.235449))
                              (goto _label_2 :!via `PlayFromStart`)))))
                      (elif (== 0 (`self.RotationIndex`))
                        (set `self.NewMirrorRotation` (0.0 10.0 13.826047))
                        (goto _label_2 :!via `PlayFromStart`)
                        (elif (== 1 (`self.RotationIndex`))
                          (set `self.NewMirrorRotation` (0.0 5.0 -70.0))
                          (goto _label_2 :!via `PlayFromStart`)
                          (elif (== 2 (`self.RotationIndex`))
                            (set `self.NewMirrorRotation` (0.0 -2.5 -10.45))
                            (goto _label_2 :!via `PlayFromStart`)
                            (else
                              (set `self.NewMirrorRotation` (0.0 -5.0 -120.0))
                              (goto _label_2 :!via `PlayFromStart`))))))))))))))))

(event `self.InteractionArea.OnComponentBeginOverlap`
  (params (OverlappedComponent :type "PrimitiveComponent Object Reference") (OtherActor :type "Actor Object Reference") (OtherComp :type "PrimitiveComponent Object Reference") (OtherBodyIndex :type Integer) (bFromSweep :type Boolean) (SweepResult :type "HitResult Structure (by ref)"))
  (cast `/Game/ThirdPerson/Blueprints/BP_ThirdPersonCharacter` OtherActor)
  (bind _returnvalue (`|CreateWidget` "/Game/Blueprints/WBP_InteractionPrompt.WBP_InteractionPrompt_C"))
  (set `self.InteractionWidget` _returnvalue)
  (`UserWidget.AddToViewport` _returnvalue 0))

(event `self.InteractionArea.OnComponentEndOverlap`
  (params (OverlappedComponent :type "PrimitiveComponent Object Reference") (OtherActor :type "Actor Object Reference") (OtherComp :type "PrimitiveComponent Object Reference") (OtherBodyIndex :type Integer))
  (cast `/Game/ThirdPerson/Blueprints/BP_ThirdPersonCharacter` OtherActor)
  (`Widget.RemoveFromParent` (`self.InteractionWidget`)))

(fn `UserConstructionScript`)