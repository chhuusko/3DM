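; Light-beam puzzle actor that bounces a traced beam off Mirror-tagged actors toward puzzle and secret targets.
; On BeginPlay and CastLight, it clears old lines and loops line traces from the Light component, reflecting off hit normals up to MaxReflections.
; Persistent debug lines serve as the beam visual.
; Target hits play sounds and call TargetHit, while the count of unique mirrors hit drives a pitched feedback sound.
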(event `self.ReceiveBeginPlay`
  (bind (_returnvalue_roll _returnvalue_pitch) (`KismetMathLibrary.BreakRotator` (`SceneComponent.K2_GetComponentRotation` (`self.Light`))))
  (`BlueprintSetLibrary.Set_Clear` (`self.HitMirrorsSet`) :!label _label)
  (`KismetSystemLibrary.FlushPersistentDebugLines`)
  (set `self.CurrentPosition` (`SceneComponent.K2_GetComponentLocation` (`self.Light`)))
  (set `self.CurrentDirection` (`KismetMathLibrary.MakeVector` 0.0 _returnvalue_pitch))
  (for _index (range (`self.MaxReflections`))
    (bind _outhit (`KismetSystemLibrary.LineTraceSingle` :`Start` (`self.CurrentPosition`) :`End` (+ (* (`self.CurrentDirection`) (`self.ReflectionDistance`)) (`self.CurrentPosition`)) :`TraceChannel` "TraceTypeQuery1" :`DrawTime` 0.0))
    (if (== _index 0)
      (bind (_bblockinghit _binitialoverlap _time _distance _location _impactpoint _normal _impactnormal _physmat _hitactor) (`GameplayStatics.BreakHitResult` _outhit))
      (`KismetSystemLibrary.DrawDebugLine` (`self.CurrentPosition`) _impactpoint (struct :`R` 0.984244 :`G` 1.0 :`A` 1.0) 1000000.0 2.0))
    (if _bblockinghit
      (if (`self.ActorHasTag` _hitactor "Mirror")
        (`BlueprintSetLibrary.Set_Add` (`self.HitMirrorsSet`) _hitactor)
        (set `self.CurrentDirection` (`KismetMathLibrary.GetReflectionVector` (`self.CurrentDirection`) _impactnormal))
        (set `self.CurrentPosition` (+ _impactpoint _impactnormal))
        (`KismetSystemLibrary.DrawDebugLine` (`self.CurrentPosition`) (+ (* (`self.CurrentDirection`) (`self.ReflectionDistance`)) (`self.CurrentPosition`)) (struct :`R` 0.984244 :`G` 1.0 :`A` 1.0) 1000000.0 2.0)
        (elif (`self.ActorHasTag` _hitactor "TargetSecret")
          (`GameplayStatics.PlaySound2D` "/Game/Audio/SecretTargetHit.SecretTargetHit" 1.0 1.0 0.0 null null)
          (`/Game/Blueprints/BP_LightTargetSecret.TargetHit` (`self.TargetSecret`))
          (elif (`self.ActorHasTag` _hitactor "TargetPuzzle")
            (`GameplayStatics.PlaySound2D` "/Game/Audio/TargetHit.TargetHit" 1.0 1.0 0.0 null null)
            (`/Game/Blueprints/BP_LightTargetPuzzle.TargetHit` (`self.TargetPuzzle`))
            (else
              (break)))))))
  (switch `int` (`BlueprintSetLibrary.Set_Length` (`self.HitMirrorsSet`))
    (:`2`
      _)
    (:`3`
      (set `self.PitchMultiplier` 1.0))
    (:`4`
      (set `self.PitchMultiplier` 1.2))
    (:`5`
      (set `self.PitchMultiplier` 1.4))
    (:`6`
      (set `self.PitchMultiplier` 1.6)))
  (`GameplayStatics.PlaySound2D` (`self.BaseSound`) 1.0 (`self.PitchMultiplier`) 0.0 null null))

(event `CastLight`
  (goto _label))

(fn `UserConstructionScript`)