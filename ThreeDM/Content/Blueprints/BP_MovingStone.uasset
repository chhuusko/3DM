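; BP_MovingStone is a stone that moves vertically when enough pressure plates are active.
; Switch events adjust an active-plate count and compare it to the required number, playing or reversing a timeline that drives the mesh's relative Z, with movement sounds on some paths.
; MoveStone plays the timeline directly, bypassing the count.
; An attached ButtonChild follows the mesh and has SetLocation called when the timeline finishes.
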(event `self.ReceiveBeginPlay`
  (`self.K2_AttachToComponent` (`self.ButtonChild`) (`self.StoneMesh`) "None" "KeepWorld" "KeepWorld" "KeepWorld" true)
  (set `self.InitialStoneLocation` (`SceneComponent.K2_GetComponentLocation` (`self.StoneMesh`))))

(event `SwitchActivated`
  (`/Engine/EditorBlueprintResources/StandardMacros.IncrementInt` (`self.PressurePlatesActive`)
    (:`  `
      (if (>= (`self.PressurePlatesActive`) (`self.PressurePlatesNeeded`))
        (`GameplayStatics.PlaySoundAtLocation` "/Game/Audio/StoneMoving1Sec.StoneMoving1Sec" (`self.InitialStoneLocation`) (struct) 1.0 1.0 0.0 null null null null :!label _label)
        (bind (_direction _stoneposition) (`Timeline|StoneMoving` :!label _label_2)
          (:`Update`
            (`SceneComponent.K2_SetRelativeLocation` (`self.StoneMesh`) (`KismetMathLibrary.MakeVector` 0.0 0.0 _stoneposition) false false))
          (:`Finished`
            (`/Game/Blueprints/BP_Button.SetLocation` (`self.ButtonChild`))))
        (else
          (goto _label_2 :!via `Reverse`))))))

(event `MoveStone`
  (`GameplayStatics.PlaySoundAtLocation` "/Game/Audio/StoneMoving1Sec.StoneMoving1Sec" (`self.InitialStoneLocation`) (struct) 1.0 1.0 0.0 null null null null)
  (goto _label_2))

(event `SwitchDeactivated`
  (`/Engine/EditorBlueprintResources/StandardMacros.DecrementInt` (`self.PressurePlatesActive`)
    (:`  `
      (if (>= (`self.PressurePlatesActive`) (`self.PressurePlatesNeeded`))
        (goto _label)
        (elif (!= (`self.PressurePlatesNeeded`) 1)
          (goto _label_2 :!via `Reverse`)
          (else
            (`GameplayStatics.PlaySoundAtLocation` "/Game/Audio/StoneMoving1Sec.StoneMoving1Sec" (0.0 0.0 0.0) (struct) 1.0 1.0 0.0 null null null null)
            (goto _label_2 :!via `Reverse`)))))))

(fn `UserConstructionScript`)