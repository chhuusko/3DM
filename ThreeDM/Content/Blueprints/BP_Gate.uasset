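; BP_Gate is a gate actor that moves its mesh by a set offset when MoveGate is called.
; BeginPlay caches the mesh's world location, and a timeline lerps from there to that location plus MoveOffset.
; MoveGate acts only while IsGateOpen is false, then sets it and flags LinkedButton as pressed, with no closing path.
; Leftover debug prints show the start location and fire on every timeline update.
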(event `self.ReceiveBeginPlay`
  (bind _output_get (set `self.InitialGateLocation` (`SceneComponent.K2_GetComponentLocation` (`self.GateMesh`))))
  (`KismetSystemLibrary.PrintString` (`KismetStringLibrary.Conv_VectorToString` _output_get)))

(event `MoveGate`
  (if (not (`self.IsGateOpen`))
    (set `self.IsGateOpen` true)
    (set `/Game/Blueprints/BP_Button.HasBeenPressed` true (`self.LinkedButton`))
    (bind (_direction _movealpha) (`Timeline|MoveTimeline` :!via `PlayFromStart`)
      (:`Update`
        (`SceneComponent.K2_SetWorldLocation` (`self.GateMesh`) (`KismetMathLibrary.VLerp` (`self.InitialGateLocation`) (+ (`self.InitialGateLocation`) (`self.MoveOffset`)) _movealpha) false false)
        (`KismetSystemLibrary.PrintString` "no")))))

(fn `UserConstructionScript`)