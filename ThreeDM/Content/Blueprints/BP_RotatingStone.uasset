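; BP_RotatingStone is a stone that rotates or slides once when triggered, with a gate-moving sound.
; BeginPlay caches the stone mesh's location and attaches ButtonChild and TargetChild to it, keeping world transforms.
; RotateStone turns the root through a half-turn of yaw, while MoveStone slides the mesh by MoveOffset.
; Each uses its own DoOnce and timeline, calling ButtonChild.SetLocation on every update.
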(event `self.ReceiveBeginPlay`
  (set `self.Initial Stone Location` (`SceneComponent.K2_GetComponentLocation` (`self.StoneMesh`)))
  (`self.K2_AttachToComponent` (`self.ButtonChild`) (`self.StoneMesh`) "None" "KeepWorld" "KeepWorld" "KeepWorld" true)
  (`self.K2_AttachToComponent` (`self.Target Child`) (`self.StoneMesh`) "None" "KeepWorld" "KeepWorld" "KeepWorld" true))

(event `RotateStone`
  (`/Engine/EditorBlueprintResources/StandardMacros.DoOnce` false
    (:`Completed`
      (`GameplayStatics.PlaySoundAtLocation` "/Game/Audio/GateMoving.GateMoving" (`self.Initial Stone Location`) (struct) 1.0 1.0 0.0 null null null null)
      (bind (_direction _opentrack) (`Timeline|Timeline`)
        (:`Update`
          (bind (_returnvalue_x _returnvalue_y _returnvalue_z) (`KismetMathLibrary.BreakVector` (`KismetMathLibrary.VLerp` (0.0 0.0 90.0) (0.0 0.0 270.0) _opentrack)))
          (`SceneComponent.K2_SetWorldRotation` (`self.DefaultSceneRoot`) (`KismetMathLibrary.MakeRotator` 0.0 0.0 _returnvalue_z) false false)
          (`/Game/Blueprints/BP_ButtonSecret.SetLocation` (`self.ButtonChild`)))))))

(event `MoveStone`
  (`/Engine/EditorBlueprintResources/StandardMacros.DoOnce` false
    (:`Completed`
      (`GameplayStatics.PlaySoundAtLocation` "/Game/Audio/GateMoving.GateMoving" (`self.Initial Stone Location`) (struct) 1.0 1.0 0.0 null null null null)
      (bind (_direction _opentrack) (`Timeline|Timeline_0`)
        (:`Update`
          (`SceneComponent.K2_SetWorldLocation` (`self.StoneMesh`) (`KismetMathLibrary.VLerp` (`self.Initial Stone Location`) (+ (`self.Initial Stone Location`) (`self.Move Offset`)) _opentrack) false false)
          (`/Game/Blueprints/BP_ButtonSecret.SetLocation` (`self.ButtonChild`)))))))

(fn `UserConstructionScript`)