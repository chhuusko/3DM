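; Stone that moves vertically when enough pressure plates are active, carrying an attached child button with it.
; Switch activation and deactivation events maintain a count of active plates and compare it to the required number.
; Meeting the threshold plays a timeline that drives the mesh's relative Z position, and falling short reverses it.
; At BeginPlay the button attaches to the stone mesh, keeping its world transform.
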(event `self.ReceiveBeginPlay`
  (`self.K2_AttachToComponent` (`self.ButtonChild`) (`self.StoneMesh`) "None" "KeepWorld" "KeepWorld" "KeepWorld" true))

(event `SwitchActivated`
  (`/Engine/EditorBlueprintResources/StandardMacros.IncrementInt` (`self.PressurePlatesActive`)
    (:`  `
      (if (>= (`self.PressurePlatesActive`) (`self.PressurePlatesNeeded`))
        (bind (_direction _stoneposition) (`Timeline|StoneMoving` :!label _label)
          (:`Update`
            (`SceneComponent.K2_SetRelativeLocation` (`self.StoneMesh`) (`KismetMathLibrary.MakeVector` 0.0 0.0 _stoneposition) false false)))
        (else
          (goto _label :!via `Reverse`))))))

(event `SwitchDeactivated`
  (`/Engine/EditorBlueprintResources/StandardMacros.DecrementInt` (`self.PressurePlatesActive`)
    (:`  `
      (if (>= (`self.PressurePlatesActive`) (`self.PressurePlatesNeeded`))
        (goto _label)
        (else
          (goto _label :!via `Reverse`))))))

(fn `UserConstructionScript`)